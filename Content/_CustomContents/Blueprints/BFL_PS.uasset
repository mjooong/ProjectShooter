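; BFL_PS is a Blueprint function library with shared helpers for score and timing.
; AddScore casts the current game mode to BP_PSGameMode and forwards the value to its AddScore, doing nothing if the cast fails.
; GetMillisecFromDateTime returns milliseconds between two DateTimes by building timespans from day, hour, minute, second and millisecond, so month and year are ignored.
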(fn `AddScore`
  (params (Value :type "Float (double-precision)"))
  (bind _asbp_psgame_mode (cast `/Game/_CustomContents/Gameplay/BP_PSGameMode` (`GameplayStatics.GetGameMode` null)))
  (`/Game/_CustomContents/Gameplay/BP_PSGameMode.AddScore` _asbp_psgame_mode (`local.Value`)))

(fn `GetMillisecFromDateTime`
  (params (Later :type "DateTime Structure") (Earlier :type "DateTime Structure"))
  (returns (Result :type "Float (double-precision)"))
  (bind (_year _month _day _hour _minute _second _millisecond) (`KismetMathLibrary.BreakDateTime` (`local.Earlier`)))
  (bind (_year_2 _month_2 _day_2 _hour_2 _minute_2 _second_2 _millisecond_2) (`KismetMathLibrary.BreakDateTime` (`local.Later`)))
  (return (- (`KismetMathLibrary.GetTotalMilliseconds` (`KismetMathLibrary.MakeTimespan` _day_2 _hour_2 _minute_2 _second_2 _millisecond_2)) (`KismetMathLibrary.GetTotalMilliseconds` (`KismetMathLibrary.MakeTimespan` _day _hour _minute _second _millisecond)))))
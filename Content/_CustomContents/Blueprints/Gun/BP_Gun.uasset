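; BP_Gun is a gun actor that fires bullets from a limited count and can be reloaded.
; Fire decrements RemainingBullets, prints the count for debugging, then spawns a BP_Bullet at the FrontOfGun transform and sets its speed to a fixed value.
; Reload restores RemainingBullets to MaxRemainingBullet; the event graph is empty, so both functions rely on external callers.
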(fn `Fire`
  (if (> (`self.RemainingBullets`) 0)
    (`/Engine/EditorBlueprintResources/StandardMacros.DecrementInt` (`self.RemainingBullets`)
      (:`  `
        (`|ExecutionSequence`
          (:`then_0`
            (`KismetSystemLibrary.PrintString` (`KismetStringLibrary.Concat_StrStr` "psgun / fire / RemainingBullets = " (`KismetStringLibrary.Conv_IntToString` (`self.RemainingBullets`)))))
          (:`then_1`
            (bind _returnvalue (`|SpawnActorFromClass` "/Game/_CustomContents/Blueprints/Gun/BP_Bullet.BP_Bullet_C" (`SceneComponent.K2_GetComponentToWorld` (`self.FrontOfGun`)) "Undefined" "MultiplyWithRoot" null null))
            (`/Game/_CustomContents/Blueprints/Gun/BP_Bullet.SetSpeed` _returnvalue 1000.0)))))))

(fn `Reload`
  (set `self.RemainingBullets` (`self.MaxRemainingBullet`)))

(fn `UserConstructionScript`)
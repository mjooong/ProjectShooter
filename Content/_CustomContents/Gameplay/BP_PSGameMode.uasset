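; BP_PSGameMode is a game mode that tracks a timed round through Ready, Playing and Ended states, along with a score.
; StartGame and EndGame act only from their expected state and record wall-clock timestamps.
; EndGame derives elapsed seconds from day-to-millisecond fields, ignoring month and year, and passes any time left under two minutes to AddScore as a bonus.
; AddScore ignores its Value input and adds zero, leaving Score unchanged.
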(fn `AddScore`
  (params (Value :type "Float (double-precision)"))
  (set `self.Score` (+ (`self.Score`) 0.0)))

(fn `EndGame`
  (locals (TimeBonus :type "Float (double-precision)"))
  (bind (_year _month _day _hour _minute _second _millisecond) (`KismetMathLibrary.BreakDateTime` (`self.StartTime`)))
  (bind (_year_2 _month_2 _day_2 _hour_2 _minute_2 _second_2 _millisecond_2) (`KismetMathLibrary.BreakDateTime` (`self.EndTime`)))
  (switch `/Game/_CustomContents/Gameplay/StateOfGame` (`self.State`)
    (:`NewEnumerator1`
      (set `self.State` "NewEnumerator2")
      (set `self.EndTime` (`KismetMathLibrary.Now`))
      (bind _output_get (set `self.ElapsedTime` (/ (- (`KismetMathLibrary.GetTotalMilliseconds` (`KismetMathLibrary.MakeTimespan` _day_2 _hour_2 _minute_2 _second_2 _millisecond_2)) (`KismetMathLibrary.GetTotalMilliseconds` (`KismetMathLibrary.MakeTimespan` _day _hour _minute _second _millisecond))) 1000.0)))
      (bind _output_get_2 (set `local.TimeBonus` (- 120.0 _output_get)))
      (if (> _output_get_2 0.0)
        (`self.AddScore` (`local.TimeBonus`))))))

(fn `StartGame`
  (switch `/Game/_CustomContents/Gameplay/StateOfGame` (`self.State`)
    (:`NewEnumerator0`
      (set `self.State` "NewEnumerator1")
      (set `self.StartTime` (`KismetMathLibrary.Now`)))))

(fn `UserConstructionScript`)